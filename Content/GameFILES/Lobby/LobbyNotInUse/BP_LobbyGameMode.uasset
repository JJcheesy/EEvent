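; Lobby game mode that gives each joining player a character at a PlayerStart.
; PostLogin records the new controller, gets its lobby controller reference through a message call and passes it to SpawnPlayer.
; SpawnPlayer refreshes the start points, increments an index, and within MaxPlayers spawns and possesses a character there, printing if that point is invalid.
; The lobby controller's InitSetup call is disconnected and never runs.
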(event `self.K2_PostLogin`
  (params (NewPlayer :type "PlayerController Object Reference"))
  (bind _output_get (set `self.connectedplayer` NewPlayer))
  (`KismetArrayLibrary.Array_AddUnique` (`self.connectedplayers`) _output_get)
  (bind _outactors (`GameplayStatics.GetAllActorsOfClass` "/Script/Engine.PlayerStart"))
  (set `self.SpawnPoints` _outactors)
  (message `/Game/GameFILES/Interface/BPI_GameInstance.GameInfoInstanceRef` (`GameplayStatics.GetGameInstance`))
  (bind _lobbypc (message `/Game/GameFILES/Lobby/LobbyNotInUse/BPI_LobbyPlayerController.LobbyPCRef` (`self.connectedplayer`)))
  (`self.Spawn Player` _lobbypc))

(event `CustomEvent_0`)

(fn `GetPlayerStartPoints`
  (bind _outactors (`GameplayStatics.GetAllActorsOfClass` "/Script/Engine.PlayerStart"))
  (set `self.SpawnPoints` _outactors))

(fn `Spawn Player`
  (params (LobbyPC :type "PlayerController Object Reference"))
  (bind _output (`|GetArrayItem` (`self.SpawnPoints`) (`self.Index`)))
  ;[1 1 1] Spawns a player and poesses a player char
  (`self.GetPlayerStartPoints`)
  (set `self.Index` (+ (`self.Index`) 1))
  (if (>= (`self.Max Players`) (`self.Index`))
    (`/Engine/EditorBlueprintResources/StandardMacros.IsValid` _output
      (:`Is Valid`
        (bind _returnvalue (`|SpawnActorFromClass` "/Game/GameFILES/Gameplay/PlayerChar.PlayerChar_C" (`self.GetTransform` _output) "AlwaysSpawn" "OverrideRootScale" null null))
        (`/Engine/EditorBlueprintResources/StandardMacros.IsValid` _returnvalue
          (:`Is Valid`
            (`Controller.Possess` LobbyPC _returnvalue))))
      (:`Is Not Valid`
        (`KismetSystemLibrary.PrintString` (`KismetSystemLibrary.GetDisplayName` _output))))))

(fn `UserConstructionScript`)